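; Player controller that places a selected static mesh where the mouse is clicked on the game's 2D plane at Y = 0.
; ProjectMousePtrToPlane deprojects the cursor into a world ray and intersects it with that plane.
; Left click spawns an ExposedStaticMeshBP there with SelectedMesh, using a quarter X scale that is noted as a workaround.
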(event Input|ActionEvents|InputActionLeftClick
  (params (Key :type Key%20Structure :default "None"))
  (:Pressed
    (bind _intersection (CallFunction|ProjectMousePtrtoPlane))
    (Game|SpawnActorfromClass "/Game/Temporary_Level/Blueprints/ExposedStaticMeshBP.ExposedStaticMeshBP_C" (Math|Transform|MakeTransform _intersection "0, 0, 0" "0.250000,1.000000,1.000000") "AdjustIfPossibleButDontSpawnIfColliding" 0 (Variables|Default|GetSelectedMesh) 0)))

(fn ConstructionScript)

(fn ProjectMousePtrtoPlane
  (bind (_worldlocation _worlddirection) (Game|Player|ConvertMouseLocationToWorldSpace))
  (return (.Intersection (Class|KismetMathLibrary|LinePlaneIntersectionOriginNormal _worldlocation (+ _worldlocation (* _worlddirection (Variables|Default|GetPlaneDist))) "0, 0, 0" "0,1.000000,0.000000"))))