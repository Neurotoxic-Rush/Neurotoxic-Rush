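; Player controller that handles the press-any-key start and the choice of which object to place, blood cell or mucous membrane.
; Play begins paused behind a prompt widget; any key unpauses, swaps in the main UI and shows the cursor.
; Two input actions or right-click cycling set the selected class and ghost mesh.
; A helper intersects the mouse ray with the Y=0 gameplay plane; spawning happens outside this Blueprint.
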(event EventBeginPlay
  (bind _returnvalue (UserInterface|CreateWidget "/Game/Temporary_Level/Blueprints/UI/AnyButtonBP.AnyButtonBP_C"))
  (UserInterface|Viewport|AddtoViewport _returnvalue 0)
  (Game|SetGamePaused true))

(event Input|ActionEvents|InputActionPressed1
  (params (Key :type Key%20Structure :default "None"))
  (:Pressed
    ;[1 1 1] for ghost, manually set
    ;;[1 1 1] Comment
    (Variables|Default|SetSelectedMesh "/Game/Temporary_Level/Shape_Cell.Shape_Cell")
    (Variables|Default|SetSelectedClass "/Game/Temporary_Level/Blueprints/Blocks/BloodCellBP.BloodCellBP_C")
    (Variables|Default|SetCurrentObjectNumber 1)))

(event Input|ActionEvents|InputActionPressed2
  (params (Key :type Key%20Structure :default "None"))
  (:Pressed
    (Variables|Default|SetSelectedMesh "/Game/StarterContent/Shapes/Shape_Cube.Shape_Cube")
    (Variables|Default|SetSelectedClass "/Game/Temporary_Level/Blueprints/Blocks/MucousMembranceBP.MucousMembranceBP_C")
    (Variables|Default|SetCurrentObjectNumber 2)))

(event Input|ActionEvents|InputActionRightClick
  (params (Key :type Key%20Structure :default "None"))
  (:Released
    (bind _output_get (Variables|Default|SetCurrentObjectNumber (+ (Variables|Default|GetCurrentObjectNumber) 1)))
    (switch int _output_get
      (:Default
        (Variables|Default|SetCurrentObjectNumber 1)
        (Variables|Default|SetSelectedMesh "/Game/Temporary_Level/Shape_Cell.Shape_Cell")
        (Variables|Default|SetSelectedClass "/Game/Temporary_Level/Blueprints/Blocks/BloodCellBP.BloodCellBP_C"))
      (:1
        (Variables|Default|SetSelectedMesh "/Game/Temporary_Level/Shape_Cell.Shape_Cell")
        (Variables|Default|SetSelectedClass "/Game/Temporary_Level/Blueprints/Blocks/BloodCellBP.BloodCellBP_C"))
      (:2
        (Variables|Default|SetSelectedMesh "/Game/StarterContent/Shapes/Shape_Cube.Shape_Cube")
        (Variables|Default|SetSelectedClass "/Game/Temporary_Level/Blueprints/Blocks/MucousMembranceBP.MucousMembranceBP_C")))))

(event Input|KeyboardEvents|AnyKey
  (params (Key :type Key%20Structure :default "None"))
  (:Pressed
    (if (Game|IsGamePaused)
      (Game|SetGamePaused false)
      (Widget|RemovefromParent (stale EventBeginPlay _returnvalue))
      ;[1 1 1] create ui
      (bind _returnvalue (UserInterface|CreateWidget "/Game/Temporary_Level/Blueprints/UI/UIWidget.UIWidget_C"))
      (UserInterface|Viewport|AddtoViewport _returnvalue 0)
      ;[1 1 1] may want to change, this shows cursor so players know where to click to make objects
      (Variables|/Script/Engine.PlayerController|SetbShowMouseCursor (Game|GetPlayerController 0) true))))

(fn ConstructionScript
  (Variables|Default|SetSelectedMesh "/Game/Temporary_Level/Shape_Cell.Shape_Cell")
  (Variables|Default|SetSelectedClass "/Game/Temporary_Level/Blueprints/Blocks/BloodCellBP.BloodCellBP_C")
  (Variables|Default|SetCurrentObjectNumber 1))

(fn ProjectMousePtrtoPlane
  (bind (_worldlocation _worlddirection) (Game|Player|ConvertMouseLocationToWorldSpace))
  (return (.Intersection (Class|KismetMathLibrary|LinePlaneIntersectionOriginNormal _worldlocation (+ _worldlocation (* _worlddirection (Variables|Default|GetPlaneDist))) "0, 0, 0" "0,1.000000,0.000000"))))