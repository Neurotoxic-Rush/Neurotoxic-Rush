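; Player Paper2D character, a brain that moves along X, jumps, and squishes on landing by swapping flipbooks and playing a throttled sound.
; Tick watches for a fall below a Z threshold and reloads the current level; the exit input quits.
; Both paths first save MainGameMode's PlayerDistance if it beats the HighScore slot.
; Both require an existing save, as a failed load cast halts them before restart or quit.
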(event Custom|Start_Idle
  (Sprite|SetFlipbook (Variables|Default|GetSprite) "/Game/Temporary_Level/Blueprints/Player/Animation/Brain_FlipBook.Brain_FlipBook"))

(event Custom|Start_Land
  (Sprite|SetFlipbook (Variables|Default|GetSprite) "/Game/Temporary_Level/Blueprints/Player/Animation/Brain_flat.Brain_flat"))

(event EventTick
  (params (DeltaSeconds :type Float%20%28single-precision%29))
  (if (< (.Z (Class|KismetMathLibrary|BreakVector3f (Transformation|GetActorLocation))) -1e+01)
    ;[1 1 1] Save High Score
    (bind _asmain_game_mode (Utilities|Casting|CastToMainGameMode (Game|GetGameMode)))
    (bind _returnvalue (SaveGame|LoadGamefromSlot "HighScore"))
    (bind _ashigh_score_save_data (Utilities|Casting|CastToHighScore_SaveData _returnvalue))
    (Math|Integer|CompareInt (Math|Conversions|ToInteger(Byte) (Variables|/Game/Temporary_Level/Blueprints/MainGameMode.MainGameMode_C|GetPlayerDistance _asmain_game_mode)) (Variables|/Game/Temporary_Level/Blueprints/HighScore_SaveData.HighScore_SaveData_C|GetHigh_Score _ashigh_score_save_data)
      (:>
        (bind _returnvalue_2 (SaveGame|CreateSaveGameObject "/Game/Temporary_Level/Blueprints/HighScore_SaveData.HighScore_SaveData_C"))
        (bind _ashigh_score_save_data_2 (Utilities|Casting|CastToHighScore_SaveData _returnvalue_2))
        (Variables|/Game/Temporary_Level/Blueprints/HighScore_SaveData.HighScore_SaveData_C|SetHigh_Score _ashigh_score_save_data_2 (Math|Conversions|ToInteger(Byte) (Variables|/Game/Temporary_Level/Blueprints/MainGameMode.MainGameMode_C|GetPlayerDistance _asmain_game_mode)))
        (SaveGame|SaveGametoSlot _ashigh_score_save_data_2 "HighScore"))
      (:==
        _)
      (:<
        _))
    (bind _returnvalue_3 (Game|GetCurrentLevelName true))
    (Game|OpenLevel(byName) (Utilities|String|StringToName _returnvalue_3))))

(event Collision|EventHit
  (params (MyComp :type Primitive%20Component%20Object%20Reference) (Other :type Actor%20Object%20Reference) (OtherComp :type Primitive%20Component%20Object%20Reference) (bSelfMoved :type Boolean) (HitLocation :type Vector :default "0, 0, 0") (HitNormal :type Vector :default "0, 0, 0") (NormalImpulse :type Vector :default "0, 0, 0") (Hit :type Hit%20Result%20Structure%20%28by%20ref%29))
  (if (> (.Z (Math|Vector|BreakVector HitNormal)) 0.0)
    (Utilities|FlowControl|Sequence
      (:then_0
        (if (not (Variables|Default|GetSquishPlaying))
          (Audio|PlaySound2D "/Game/Temporary_Level/squish.squish" 0.8 1.0 0.4 0 0 false)
          (Variables|Default|SetSquishPlaying true)
          (Utilities|FlowControl|Delay 0.533)
          (Variables|Default|SetSquishPlaying false)))
      (:then_1
        (CallFunction|StartLand)
        (Variables|Default|SetIsIdle false)
        (Utilities|FlowControl|Delay 0.5)
        (if (not (Variables|Default|GetIsIdle))
          (Variables|Default|SetIsIdle true)
          (CallFunction|StartIdle))))))

(event Input|ActionEvents|InputActionJump
  (params (Key :type Key%20Structure :default "None"))
  (:Pressed
    (Character|Jump)
    (if (not (Variables|Default|GetIsIdle))
      (Variables|Default|SetIsIdle true)
      (CallFunction|StartIdle)))
  (:Released
    (Character|StopJumping)))

(event Input|ActionEvents|InputActionExitGame
  (params (Key :type Key%20Structure :default "None"))
  (:Pressed
    ;[1 1 1] Save High Score
    (bind _asmain_game_mode (Utilities|Casting|CastToMainGameMode (Game|GetGameMode)))
    (bind _returnvalue (SaveGame|LoadGamefromSlot "HighScore"))
    (bind _ashigh_score_save_data (Utilities|Casting|CastToHighScore_SaveData _returnvalue))
    (Math|Integer|CompareInt (Math|Conversions|ToInteger(Byte) (Variables|/Game/Temporary_Level/Blueprints/MainGameMode.MainGameMode_C|GetPlayerDistance _asmain_game_mode)) (Variables|/Game/Temporary_Level/Blueprints/HighScore_SaveData.HighScore_SaveData_C|GetHigh_Score _ashigh_score_save_data)
      (:>
        (bind _returnvalue_2 (SaveGame|CreateSaveGameObject "/Game/Temporary_Level/Blueprints/HighScore_SaveData.HighScore_SaveData_C"))
        (bind _ashigh_score_save_data_2 (Utilities|Casting|CastToHighScore_SaveData _returnvalue_2))
        (Variables|/Game/Temporary_Level/Blueprints/HighScore_SaveData.HighScore_SaveData_C|SetHigh_Score _ashigh_score_save_data_2 (Math|Conversions|ToInteger(Byte) (Variables|/Game/Temporary_Level/Blueprints/MainGameMode.MainGameMode_C|GetPlayerDistance _asmain_game_mode)))
        (SaveGame|SaveGametoSlot _ashigh_score_save_data_2 "HighScore"))
      (:==
        _)
      (:<
        _))
    (Game|QuitGame 0 "Quit" false)))

(event Input|AxisEvents|InputAxisHorizontalMovement
  (params (AxisValue :type Float%20%28single-precision%29))
  (Pawn|Input|AddMovementInput "1.000000, 0, 0" (* AxisValue 1.0) false))

(fn ConstructionScript)