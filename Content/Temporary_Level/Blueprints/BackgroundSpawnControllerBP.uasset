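; Controller actor that endlessly spawns background pieces ahead of the player as they move along X, apparently for a side-scroller.
; Each tick, when the player nears the furthest background X, it advances that X by a fixed width and spawns a BackgroundBP there at hard-coded Y, Z, rotation and scale.
; GetParallaxShift returns a small opposite-direction offset from the player's X velocity for parallax scrolling.
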(event EventTick
  (params (DeltaSeconds :type Float%20%28single-precision%29))
  (Math|Float|CompareFloat (.x (Transformation|GetActorLocation (Game|GetPlayerCharacter 0))) (- (Variables|Default|GetFurthestBackgroundX) 3.3e+03)
    (:>
      (bind _output_get (Variables|Default|SetFurthestBackgroundX (+ (Variables|Default|GetFurthestBackgroundX) 1.65e+03)))
      (Game|SpawnActorfromClass "/Game/Temporary_Level/Blueprints/BackgroundBP.BackgroundBP_C" (Math|Transform|MakeTransform (Math|Vector|MakeVector _output_get -1e+02 4.5e+02) "0.000000, 0,90.000000" "16.666670,9.100000,1.000000") "AdjustIfPossibleButAlwaysSpawn" 0 0))))

(fn ConstructionScript)

(fn GetParallaxShift
  (return (* (.x (Pawn|Components|CharacterMovement|GetLastUpdateVelocity (Variables|/Script/Engine.Character|GetCharacterMovement (Game|GetPlayerCharacter 0)))) -0.02)))