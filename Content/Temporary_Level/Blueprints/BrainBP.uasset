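; BrainBP is a brain actor moved by player input through physics forces on its BrainCollider component.
; The MoveLeft and MoveRight axis events both push the collider along its own forward vector, scaled by the axis value, so direction depends on that value's sign.
; Force is applied as an acceleration change, ignoring mass, and no other logic is active.
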(event EventBeginPlay)

(event Collision|EventActorBeginOverlap
  (params (OtherActor :type Actor%20Object%20Reference)))

(event EventTick
  (params (DeltaSeconds :type Float%20%28single-precision%29)))

(event Input|AxisEvents|InputAxisMoveRight
  (params (AxisValue :type Float%20%28single-precision%29))
  (Physics|AddForce (Variables|Default|GetBrainCollider) (* (* AxisValue 6e+02) (Math|Vector|GetForwardVector (Variables|Default|GetBrainCollider))) "None" true))

(event Input|AxisEvents|InputAxisMoveLeft
  (params (AxisValue :type Float%20%28single-precision%29))
  (Physics|AddForce (Variables|Default|GetBrainCollider) (* (* AxisValue 6e+02) (Math|Vector|GetForwardVector (Variables|Default|GetBrainCollider))) "None" true))

(fn ConstructionScript)