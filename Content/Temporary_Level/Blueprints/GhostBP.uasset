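; GhostBP is a placement preview that follows the mouse with the player's selected mesh and shows whether the spot is occupied.
; Every Tick, it copies SelectedMesh from PlayerControllerBP and moves the Ghost component to that controller's mouse-to-plane projection.
; An overlap query against WorldDynamic and WorldStatic objects at that position switches the material to red when blocked and green when clear.
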(event EventTick
  (params (DeltaSeconds :type Float%20%28single-precision%29))
  (bind _asplayer_controller_bp (Utilities|Casting|CastToPlayerControllerBP (Game|GetPlayerController 0)))
  (Components|StaticMesh|SetStaticMesh (Variables|Default|GetGhost) (Variables|/Game/Temporary_Level/Blueprints/PlayerControllerBP.PlayerControllerBP_C|GetSelectedMesh _asplayer_controller_bp))
  (bind _intersection (Default|ProjectMousePtrtoPlane _asplayer_controller_bp))
  (Transformation|SetWorldLocation (Variables|Default|GetGhost) _intersection false false)
  (bind _returnvalue (Collision|ComponentOverlapActors (Variables|Default|GetGhost) (Math|Conversions|ToTransform(Vector) _intersection) (Utilities|Array|MakeArray "ObjectTypeQuery2" "ObjectTypeQuery1") 0))
  (if _returnvalue
    (Rendering|Material|SetMaterial (Variables|Default|GetGhost) 0 "/Game/Temporary_Level/Materials/M_RedGhost.M_RedGhost")
    (else
      (Rendering|Material|SetMaterial (Variables|Default|GetGhost) 0 "/Game/Temporary_Level/Materials/M_GreenGhost.M_GreenGhost"))))

(fn ConstructionScript)