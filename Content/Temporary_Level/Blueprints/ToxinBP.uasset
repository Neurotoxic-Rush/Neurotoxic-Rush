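; ToxinBP is a toxin hazard that chases the player along the X axis and restarts the level when PaperBP begins overlapping it.
; Each tick it sets its Cube's physics velocity from the X distance to the player times ToxinSpeed, so it moves faster when farther behind.
; It shows an alert widget while off-screen, using WasRecentlyRendered.
; Actors leaving its overlap are destroyed, except GhostBP.
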(event EventBeginPlay
  ;[1 1 1] alert icon logic setup
  (bind _returnvalue (UserInterface|CreateWidget "/Game/Temporary_Level/Blueprints/UI/ToxinAlertUIWidget.ToxinAlertUIWidget_C"))
  (bind _output_get (Variables|Default|SetToxinAlertWidget _returnvalue))
  (UserInterface|Viewport|AddtoViewport _output_get 0)
  (Widget|SetVisibility _output_get "Hidden"))

(event Collision|EventActorBeginOverlap
  (params (OtherActor :type Actor%20Object%20Reference))
  (Utilities|Casting|CastToPaperBP OtherActor)
  (bind _returnvalue (Game|GetCurrentLevelName true))
  (Game|OpenLevel(byName) (Utilities|String|StringToName _returnvalue)))

(event EventTick
  (params (DeltaSeconds :type Float%20%28single-precision%29))
  (bind _toxinalertwidget (Variables|Default|GetToxinAlertWidget))
  (Physics|SetPhysicsLinearVelocity (Variables|Default|GetCube) (Math|Vector|MakeVector (* (- (.x (Transformation|GetActorLocation (Game|GetPlayerCharacter 0))) (.x (Transformation|GetActorLocation))) (Variables|Default|GetToxinSpeed)) 0.0 0.0) false "None")
  (if (Class|Actor|WasRecentlyRendered 0.2)
    (Widget|SetVisibility _toxinalertwidget "Hidden")
    (else
      (Widget|SetVisibility _toxinalertwidget "Visible"))))

(event Collision|EventActorEndOverlap
  (params (OtherActor :type Actor%20Object%20Reference))
  (Utilities|Casting|CastToGhostBP OtherActor
    (:CastFailed
      (Actor|DestroyActor OtherActor))))

(fn ConstructionScript)