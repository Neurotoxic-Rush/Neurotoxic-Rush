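; Obstacle spawner that keeps generating flat blocks ahead of the player along the X axis, as in an endless side-scrolling level.
; Each Tick, when the player comes within a trigger distance of the furthest block X, it spawns a SimpleFlatBlockBP in the next slot and advances that X by the slot size.
; Height and length are randomized within limits; an unconnected WIP branch would add raised ceiling blocks.
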(event EventTick
  (params (DeltaSeconds :type Float%20%28single-precision%29))
  (Math|Float|CompareFloat (.X (Class|KismetMathLibrary|BreakVector3f (Transformation|GetActorLocation (Game|GetPlayerCharacter 0)))) (- (Variables|Default|Getfurthest_block_x) (Variables|Default|Getdistance_to_trigger_spawn))
    (:>
      (Game|SpawnActorfromClass "/Game/Temporary_Level/Blueprints/SimpleFlatBlockBP.SimpleFlatBlockBP_C" (Math|Transform|MakeTransform (Math|Vector|MakeVector (+ (Variables|Default|Getfurthest_block_x) (/ (Variables|Default|Getblock_slot_size) 2.0)) 0.0 (Math|Random|RandomFloatinRange 0.0 (Variables|Default|Getmax_spawn_height))) "0, 0, 0" (Math|Vector|MakeVector (Math|Random|RandomFloatinRange 1.5 (/ (Variables|Default|Getblock_slot_size) 1e+02)) 1.0 3.0)) "AdjustIfPossibleButAlwaysSpawn" 0 0)
      (Variables|Default|Setfurthest_block_x (+ (Variables|Default|Getfurthest_block_x) (Variables|Default|Getblock_slot_size))))))

(fn ConstructionScript)