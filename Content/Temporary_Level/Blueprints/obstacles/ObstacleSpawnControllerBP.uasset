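; Procedural level spawner that extends the ground along X ahead of the player.
; Each Tick, when the player nears FurthestBlockX, it spawns a piece there and advances that marker by the piece's length.
; The opening stretch uses only flat blocks of random height, then obstacles are randomly mixed in.
; MainGameMode's TimeElapsed progressively unlocks three obstacle sets; an unfinished ceiling-block spawn is left disconnected.
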(event EventTick
  (params (DeltaSeconds :type Float%20%28single-precision%29))
  (bind _obstacles_set2 (Variables|Default|Getobstacles_set2))
  (bind _obstacles_set3 (Variables|Default|Getobstacles_set3))
  (bind _obstacles_set1 (Variables|Default|Getobstacles_set1))
  (bind _distance_to_trigger_spawn (Variables|Default|Getdistance_to_trigger_spawn))
  (Math|Float|CompareFloat (.X (Class|KismetMathLibrary|BreakVector3f (Transformation|GetActorLocation (Game|GetPlayerCharacter 0)))) (- (Variables|Default|Getfurthest_block_x) _distance_to_trigger_spawn)
    (:>
      ;[1 1 1] Only Spawn normal blocks within a range
      (Math|Float|CompareFloat (Variables|Default|Getfurthest_block_x) (* _distance_to_trigger_spawn 2.0)
        (:>
          ;[1 1 1] Randomly chose between obstacles or normal ground
          (Math|Float|CompareFloat (Math|Random|RandomFloatinRange 0.0 1e+01) 7.0 :!label _label
            (:>
              (bind _asmain_game_mode (Utilities|Casting|CastToMainGameMode (Game|GetGameMode) :!label _label_2))
              (if (<= (Variables|/Game/Temporary_Level/Blueprints/MainGameMode.MainGameMode_C|GetTimeElapsed _asmain_game_mode) 20)
                (bind _returnvalue (Game|SpawnActorfromClass (Utilities|Array|Get(acopy) _obstacles_set1 (Math|Random|RandomIntegerinRange 0 (- (Utilities|Array|Length _obstacles_set1) 1))) (Math|Transform|MakeTransform (Math|Vector|MakeVector (Variables|Default|Getfurthest_block_x) 0.0 0.0)) "AdjustIfPossibleButAlwaysSpawn" 0 0 :!label _label_3))
                (bind _asobstacle_parent_class (Utilities|Casting|CastToObstacle_Parent_Class _returnvalue))
                (Variables|Default|Setfurthest_block_x (+ (Variables|Default|Getfurthest_block_x) (Variables|/Game/Temporary_Level/Blueprints/obstacles/Obstacle_Parent_Class.Obstacle_Parent_Class_C|GetLength _asobstacle_parent_class)))
                (elif (<= (Variables|/Game/Temporary_Level/Blueprints/MainGameMode.MainGameMode_C|GetTimeElapsed _asmain_game_mode) 50)
                  ;[1 1 1] Randomly choose between set1 & set2
                  (Math|Float|CompareFloat (Math|Random|RandomFloatinRange 0.0 1e+01) 5.0
                    (:>
                      (goto _label_3))
                    (:==
                      _)
                    (:<
                      _))
                  (bind _returnvalue_2 (Game|SpawnActorfromClass (Utilities|Array|Get(acopy) _obstacles_set2 (Math|Random|RandomIntegerinRange 0 (- (Utilities|Array|Length _obstacles_set2) 1))) (Math|Transform|MakeTransform (Math|Vector|MakeVector (Variables|Default|Getfurthest_block_x) 0.0 0.0)) "AdjustIfPossibleButAlwaysSpawn" 0 0 :!label _label_4))
                  (bind _asobstacle_parent_class_2 (Utilities|Casting|CastToObstacle_Parent_Class _returnvalue_2))
                  (Variables|Default|Setfurthest_block_x (+ (Variables|Default|Getfurthest_block_x) (Variables|/Game/Temporary_Level/Blueprints/obstacles/Obstacle_Parent_Class.Obstacle_Parent_Class_C|GetLength _asobstacle_parent_class_2)))
                  (else
                    ;[1 1 1] Randomly choose between set1 & set2 &set3
                    (Math|Float|CompareFloat (Math|Random|RandomFloatinRange 0.0 1e+01) 5.0
                      (:>
                        (Math|Float|CompareFloat (Math|Random|RandomFloatinRange 0.0 1e+01) 5.0 :!label _label_5
                          (:>
                            (goto _label_3))
                          (:==
                            (goto _label_4))
                          (:<
                            (goto _label_4))))
                      (:==
                        (goto _label_5))
                      (:<
                        (bind _returnvalue_3 (Game|SpawnActorfromClass (Utilities|Array|Get(acopy) _obstacles_set3 (Math|Random|RandomIntegerinRange 0 (- (Utilities|Array|Length _obstacles_set3) 1))) (Math|Transform|MakeTransform (Math|Vector|MakeVector (Variables|Default|Getfurthest_block_x) 0.0 0.0)) "AdjustIfPossibleButAlwaysSpawn" 0 0))
                        (bind _asobstacle_parent_class_3 (Utilities|Casting|CastToObstacle_Parent_Class _returnvalue_3))
                        (Variables|Default|Setfurthest_block_x (+ (Variables|Default|Getfurthest_block_x) (Variables|/Game/Temporary_Level/Blueprints/obstacles/Obstacle_Parent_Class.Obstacle_Parent_Class_C|GetLength _asobstacle_parent_class_3)))))))))
            (:==
              (goto _label_2))
            (:<
              (Game|SpawnActorfromClass "/Game/Temporary_Level/Blueprints/obstacles/SimpleFlatBlockBP.SimpleFlatBlockBP_C" (Math|Transform|MakeTransform (Math|Vector|MakeVector (+ (Variables|Default|Getfurthest_block_x) (/ (Variables|Default|Getblock_slot_size) 2.0)) 0.0 0.0) "0, 0, 0" (Math|Vector|MakeVector (/ (Variables|Default|Getblock_slot_size) 1e+02) 1.0 (Math|Random|RandomFloatinRange 1.0 (Variables|Default|Getmax_spawn_scale)))) "AdjustIfPossibleButAlwaysSpawn" 0 0 :!label _label_6)
              (Variables|Default|Setfurthest_block_x (+ (Variables|Default|Getfurthest_block_x) (Variables|Default|Getblock_slot_size))))))
        (:==
          (goto _label))
        (:<
          (goto _label_6))))))

(fn ConstructionScript)