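; BloodCellBP is a temporary blood cell actor that counts down a lifetime and destroys itself when it runs out.
; Each Tick decrements TimeLeft and, while time remains, runs a guarded blink cycle that shows the actor, waits, hides it briefly, then releases the Blinking flag.
; Both delays scale with TimeLeft, so the flicker speeds up as expiry nears, with the hidden phase a tenth of the visible one.
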(event EventTick
  (params (DeltaSeconds :type Float%20%28single-precision%29))
  (bind _output_get (Variables|Default|Settime_left (- (Variables|Default|Gettime_left) DeltaSeconds)))
  (Math|Float|CompareFloat _output_get 0.0
    (:>
      (if (not (Variables|Default|Getblinking)) :!label _label
        (Variables|Default|Setblinking true)
        (Rendering|SetActorHiddenInGame false)
        (Utilities|FlowControl|Delay (/ (Variables|Default|Gettime_left) 3.0))
        (Rendering|SetActorHiddenInGame true)
        (Utilities|FlowControl|Delay (/ (/ (Variables|Default|Gettime_left) 3.0) 1e+01))
        (Variables|Default|Setblinking false)))
    (:==
      (goto _label))
    (:<
      (Actor|DestroyActor))))

(fn ConstructionScript)