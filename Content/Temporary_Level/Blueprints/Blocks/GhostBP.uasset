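; GhostBP is a placement preview that follows the mouse and spawns the selected block class on left click.
; Each tick it takes the selected mesh from PlayerControllerBP and moves it to the cursor's projected point on a plane.
; An overlap query against PaperBP actors tints the ghost red when blocked, green otherwise.
; Clicking spawns only when unblocked, at the ghost's location with fixed rotation and scale.
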(event EventTick
  (params (DeltaSeconds :type Float%20%28single-precision%29))
  (bind _asplayer_controller_bp (Utilities|Casting|CastToPlayerControllerBP (Game|GetPlayerController 0)))
  (Components|StaticMesh|SetStaticMesh (Variables|Default|GetGhost) (Variables|/Game/Temporary_Level/Blueprints/Player/PlayerControllerBP.PlayerControllerBP_C|GetSelectedMesh _asplayer_controller_bp))
  (bind _intersection (Default|ProjectMousePtrtoPlane _asplayer_controller_bp))
  (Transformation|SetWorldLocation (Variables|Default|GetGhost) _intersection false false)
  (bind _returnvalue (Collision|ComponentOverlapActors (Variables|Default|GetGhost) (Math|Conversions|ToTransform(Vector) _intersection) (Utilities|Array|MakeArray "ObjectTypeQuery2" "ObjectTypeQuery1") "/Game/Temporary_Level/Blueprints/Player/PaperBP.PaperBP_C"))
  (bind _output_get (Variables|Default|Setoverlapping _returnvalue))
  (if _output_get
    (Rendering|Material|SetMaterial (Variables|Default|GetGhost) 0 "/Game/Temporary_Level/Materials/M_RedGhost.M_RedGhost")
    (else
      (Rendering|Material|SetMaterial (Variables|Default|GetGhost) 0 "/Game/Temporary_Level/Materials/M_GreenGhost.M_GreenGhost"))))

(event Input|ActionEvents|InputActionLeftClick
  (params (Key :type Key%20Structure))
  (:Pressed
    (if (not (Variables|Default|Getoverlapping))
      (bind _asplayer_controller_bp (Utilities|Casting|CastToPlayerControllerBP (Game|GetPlayerController 0)))
      (Game|SpawnActorfromClass (Variables|/Game/Temporary_Level/Blueprints/Player/PlayerControllerBP.PlayerControllerBP_C|GetSelectedClass _asplayer_controller_bp) (Math|Transform|MakeTransform (Transformation|GetWorldLocation (Variables|Default|GetGhost)) "0, 0, 0" "1.000000,0.500000,1.000000") "AlwaysSpawn" 0 0))))

(fn ConstructionScript)