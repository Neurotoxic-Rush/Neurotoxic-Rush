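; Obstacle track piece that extends the level by spawning a follow-on piece when a BrainBP actor enters its trigger box.
; The first such overlap sets a one-shot flag and spawns a random class from ObstaclesList at the ArrowEnd transform, chaining pieces end to end.
; After a fixed delay, the piece destroys itself to clear itself from the level.
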(event OnComponentBeginOverlap(Box)
  (params (OverlappedComponent :type Primitive%20Component%20Object%20Reference) (OtherActor :type Actor%20Object%20Reference) (OtherComp :type Primitive%20Component%20Object%20Reference) (OtherBodyIndex :type Integer) (bFromSweep :type Boolean) (SweepResult :type Hit%20Result%20Structure%20%28by%20ref%29))
  (bind _obstacles_list (Variables|Default|GetObstacles_List))
  (Utilities|Casting|CastToBrainBP OtherActor)
  (if (not (Variables|Default|Gettriggered))
    (Variables|Default|Settriggered true)
    (Game|SpawnActorfromClass (Utilities|Array|Get(acopy) _obstacles_list (Math|Random|RandomIntegerinRange 0 (Utilities|Array|LastIndex _obstacles_list))) (Transformation|GetWorldTransform (Variables|Default|GetArrowEnd)) "Undefined" 0 0)
    (Utilities|FlowControl|Delay 1e+01)
    (Actor|DestroyActor)))

(event EventBeginPlay)

(event Collision|EventActorBeginOverlap
  (params (OtherActor :type Actor%20Object%20Reference)))

(event EventTick
  (params (DeltaSeconds :type Float%20%28single-precision%29)))

(fn ConstructionScript)